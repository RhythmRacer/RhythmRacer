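; Base player vehicle with arcade-style movement, driven by acceleration and turning input and tuned through VehicleData.
; Input eases CurrentSpeed toward max or zero with FInterpTo, while steering yaws the actor, scaled by a speed-based curve.
; Tick decelerates without throttle, then moves the actor forward with a swept offset.
; Movement audio stops when playing below a speed threshold, but starts whenever idle, regardless of speed.
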(event EventTick
  (params (DeltaSeconds :type Float%20%28single-precision%29))
  ;[0.15 0.15 0.15 0.5] Comment
  (Utilities|FlowControl|Sequence
    (:then_0
      ;[0.15 0.15 0.15 0.5] DeccelerationHandling
      (if (not (Variables|Control|GetAcceleratedOnLastTick))
        (Variables|Control|SetcurrentSpeed (Math|Interpolation|FInterpTo (Variables|Control|GetcurrentSpeed) 0.0 (Utilities|Time|GetWorldDeltaSeconds) (.decelerationrate (Variables|Developer|GetvehicleData))))))
    (:then_1
      ;[0.15 0.15 0.15 0.5] Update Position (Keep as last)
      (Tick|UpdatePosition)
      (Variables|Control|SetAcceleratedOnLastTick false))
    (:then_2
      ;[0.15 0.15 0.15 0.5] Movement Audio
      (Utilities|EvaluateMovementSound))))

(event Custom|Action_Accelerate
  (params (Acceleration%20Input :type Float%20%28double-precision%29))
  (Action|Acceleration Acceleration%20Input))

(event Custom|Action_Turning
  (params (Input :type Float%20%28double-precision%29))
  (Action|Steer Input))

(fn ConstructionScript)

(fn UpdatePosition
  (Utilities|FlowControl|Sequence
    (:then_0
      ;[0.15 0.15 0.15 0.5] Get Actor Forward
      (LocalVariables|SetForward (Transformation|GetActorForwardVector)))
    (:then_1
      ;[0.15 0.15 0.15 0.5] Figure out where it should move to
      (LocalVariables|SetOffset (* (LocalVariables|GetForward) (Variables|Control|GetcurrentSpeed) (Utilities|Time|GetWorldDeltaSeconds))))
    (:then_2
      ;[0.15 0.15 0.15 0.5] Apply Offset
      (Transformation|AddActorWorldOffset self (LocalVariables|GetOffset) true))))

(fn Steer
  (params (Steering%20Input :type Float%20%28double-precision%29))
  (bind _returnvalue (Transformation|GetActorRotation))
  (LocalVariables|SetSteeringInput Steering%20Input)
  (Utilities|FlowControl|Sequence
    (:then_0
      ;[0.15 0.15 0.15 0.5] Figure Out Turn Strength
      (LocalVariables|SetTurnMultiplier (Math|Curves|GetFloatValue (.turnspeedcruve (Variables|Developer|GetvehicleData)) (Variables|Control|GetcurrentSpeed))))
    (:then_1
      ;[0.15 0.15 0.15 0.5] Calculate rotation ammount
      (LocalVariables|SetTurnAmmount (* (LocalVariables|GetSteeringInput) (.steeringrate (Variables|Developer|GetvehicleData)) (LocalVariables|GetTurnMultiplier) (Utilities|Time|GetWorldDeltaSeconds))))
    (:then_2
      ;[0.15 0.15 0.15 0.5] Apply Turn
      (Transformation|SetActorRotation (Math|Rotator|MakeRotator (.roll _returnvalue) (.pitch _returnvalue) (+ (.yaw _returnvalue) (LocalVariables|GetTurnAmmount)))))))

(fn Acceleration
  (params (Input :type Float%20%28double-precision%29))
  (bind _vehicledata (Variables|Developer|GetvehicleData))
  ;[0.15 0.15 0.15 0.5] Check if accelerating or decelerating
  (if (> Input 0.0)
    ;[0.15 0.15 0.15 0.5] AccelerationHandling
    (Variables|Control|SetcurrentSpeed (Math|Interpolation|FInterpTo (Variables|Control|GetcurrentSpeed) (.maxspeed _vehicledata) (Utilities|Time|GetWorldDeltaSeconds) (.accelerationrate _vehicledata)))
    (Variables|Control|SetAcceleratedOnLastTick true)
    (else
      ;[0.15 0.15 0.15 0.5] DeccelerationHandling
      (Variables|Control|SetcurrentSpeed (Math|Interpolation|FInterpTo (Variables|Control|GetcurrentSpeed) 0.0 (Utilities|Time|GetWorldDeltaSeconds) (.decelerationrate (Variables|Developer|GetvehicleData)))))))