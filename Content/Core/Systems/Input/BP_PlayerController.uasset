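; Player controller that routes driving input to the possessed vehicle.
; On BeginPlay it adds the driving Enhanced Input mapping context and caches the controlled pawn as a BP_BaseVehicle, printing a warning if the cast fails.
; Acceleration and turning input actions forward their values to that vehicle's accelerate and turning functions.
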(event EventBeginPlay
  (bind _self self)
  (Input|AddMappingContext (PlayerController|LocalPlayerSubsystems|GetEnhancedInputLocalPlayerSubsystem _self) "/Game/Core/Systems/Input/IMC_Driving.IMC_Driving" 0 "(bIgnoreAllPressedKeysUntilRelease=True,bForceImmediately=False,bNotifyUserSettings=False)")
  (bind _asbp_base_vehicle (Utilities|Casting|CastToBP_BaseVehicle (Pawn|GetControlledPawn _self))
    (:then
      (Variables|Default|SetPlayer%20Pawn _asbp_base_vehicle))
    (:CastFailed
      (Development|PrintText "Player Controller: Attatched Pawn is not of type BP_Vehicle"))))

(event Input|EnhancedActionEvents|EnhancedInputActionIA_Acceleration
  (params (ActionValue :type Float%20%28double-precision%29) (ElapsedSeconds :type Float%20%28double-precision%29) (TriggeredSeconds :type Float%20%28double-precision%29) (InputAction :type Input%20Action%20Object%20Reference :default "/Game/Core/Systems/Input/IA_Acceleration.IA_Acceleration"))
  (Default|ActionAccelerate (Variables|Default|GetPlayer%20Pawn) ActionValue))

(event Input|EnhancedActionEvents|EnhancedInputActionIA_Turning
  (params (ActionValue :type Float%20%28double-precision%29) (ElapsedSeconds :type Float%20%28double-precision%29) (TriggeredSeconds :type Float%20%28double-precision%29) (InputAction :type Input%20Action%20Object%20Reference :default "/Game/Core/Systems/Input/IA_Turning.IA_Turning"))
  (Default|ActionTurning (Variables|Default|GetPlayer%20Pawn) ActionValue))

(fn ConstructionScript)